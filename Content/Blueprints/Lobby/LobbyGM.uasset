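; Lobby game mode that sets up joining players and keeps everyone's lobby information in sync.
; On login, the server registers the controller, initializes its lobby menu and possesses a new 0_Base character at a random PlayerStart.
; EveryoneUpdate then pushes player info, counts and available characters to all controllers, setting CanWeStart per player by character choice, so the last player decides.
; Launch, character swap, kick-list and cannot-start events are empty stubs.
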(event `self.K2_PostLogin`
  (params (NewPlayer :type "PlayerController Object Reference"))
  ;[1 1 1] Initial setup, occurs on event post login, handles lobby set up on player controller and spawns player
  (`/Engine/EditorBlueprintResources/ActorMacros.Switch Has Authority`
    (:`Authority`
      (`KismetArrayLibrary.Array_Add` (`self.AllPlayerControllers`) NewPlayer)
      (bind _outactors (`GameplayStatics.GetAllActorsOfClass` "/Script/Engine.PlayerStart"))
      (set `self.SpawnPoints` _outactors)
      (bind _asbp_game_info_instance (cast `/Game/Blueprints/AllLevels/BP_GameInfoInstance` (`GameplayStatics.GetGameInstance`)))
      (set `self.ServerName` (`/Game/Blueprints/AllLevels/BP_GameInfoInstance.ServerName` _asbp_game_info_instance))
      (set `self.MaxPlayers` (`/Game/Blueprints/AllLevels/BP_GameInfoInstance.MaxPlayers` _asbp_game_info_instance))
      (bind _aslobby_pc (cast `/Game/Blueprints/Lobby/LobbyPC` NewPlayer))
      (`/Game/Blueprints/Lobby/LobbyPC.InitialSetup` _aslobby_pc)
      (`/Game/Blueprints/Lobby/LobbyPC.SetupLobbyMenu` _aslobby_pc (`self.ServerName`))
      (`/Game/Blueprints/Lobby/LobbyPC.UpdateLobbySettings` _aslobby_pc (`self.GM_MapImage`) (`self.GM_MapName`) (`self.GM_MapTime`))
      (`self.RespawnPlayer` NewPlayer))))

(event `RespawnPlayer`
  (params (PlayerController :type "PlayerController Object Reference"))
  (bind _returnvalue (`Controller.K2_GetPawn` PlayerController))
  (bind _spawnpoints (`self.SpawnPoints`))
  ;[1 1 1] Spawn player as base chacater when they arrive at the lobby
  (`/Engine/EditorBlueprintResources/StandardMacros.IsValid` _returnvalue
    (:`Is Valid`
      (`self.K2_DestroyActor` _returnvalue))
    (:`Is Not Valid`
      _))
  (bind _returnvalue_2 (`|SpawnActorFromClass` "/Game/Blueprints/Characters/0_Base.0_Base_C" (`self.GetTransform` (`KismetArrayLibrary.Array_Get` _spawnpoints (`KismetMathLibrary.RandomIntegerInRange` 0 (- (`KismetArrayLibrary.Array_Length` _spawnpoints) 1)))) "Undefined" "OverrideRootScale"))
  (`Controller.Possess` PlayerController _returnvalue_2)
  (`self.EveryoneUpdate`))

(event `EveryoneUpdate`
  (bind _allplayercontrollers (`self.AllPlayerControllers`))
  ;[1 1 1] Updates all connect players lobby information when called
  (set `self.CurrentPlayers` (`KismetArrayLibrary.Array_Length` (`self.AllPlayerControllers`)))
  (if (> (`self.CurrentPlayers`) 0)
    (`KismetArrayLibrary.Array_Clear` (`self.ConnectedPlayers`))
    (for _array_element _allplayercontrollers
      (bind _aslobby_pc (cast `/Game/Blueprints/Lobby/LobbyPC` _array_element))
      (`KismetArrayLibrary.Array_Add` (`self.ConnectedPlayers`) (`/Game/Blueprints/Lobby/LobbyPC.PlayerSettings` _aslobby_pc))
      (`/Game/Blueprints/Lobby/LobbyPC.UpdateNumberOfPlayers` _aslobby_pc (`self.CurrentPlayers`) (`self.MaxPlayers`)))
    (for _array_element_2 _allplayercontrollers
      (bind _aslobby_pc_2 (cast `/Game/Blueprints/Lobby/LobbyPC` _array_element_2))
      (`/Game/Blueprints/Lobby/LobbyPC.AddPlayerInfo` _aslobby_pc_2 (`self.ConnectedPlayers`))
      (`/Game/Blueprints/Lobby/LobbyPC.UpdateAvailableCharacters` _aslobby_pc_2 (`self.AvailableCharacters`))
      (`self.AddToKickList`))
    (for _array_element_3 (`self.ConnectedPlayers`)
      (if (== (`.MyPlayerCharacter_8_1ED4DE73411DC29507A1B7907C28D4D9` (break `/Game/Blueprints/AllLevels/PlayerInfo` _array_element_3)) "/Game/Blueprints/Characters/0_Base.0_Base_C")
        (set `self.CanWeStart?` false)
        (`self.CannotStartGame`)
        (else
          (set `self.CanWeStart?` true))))))

(event `LaunchTheGame`)

(event `CannotStartGame`)

(event `SwapCharacter`
  (params (PlayerController :type "PlayerController Object Reference") (CharacterClass :type "Character Class Reference") (`ChangedStatus?` :type Boolean)))

(event `AddToKickList`)

(fn `UserConstructionScript`)